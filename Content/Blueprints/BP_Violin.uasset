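; BP_Violin is a violin pickup that moves vertically between two heights and grants the viola to the player character.
; On box overlap it sets HasViola, shows the character's Violin, destroys itself, calls ViolaControls and plays a pluck sound.
; A timeline started on BeginPlay, with its rate set from a duration variable, lerps the actor's Z.
; A separate custom event with an overlap signature sets the character's respawn location to this actor's position.
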(event `self.Box.OnComponentBeginOverlap`
  (params (OverlappedComponent :type "PrimitiveComponent Object Reference") (OtherActor :type "Actor Object Reference") (OtherComp :type "PrimitiveComponent Object Reference") (OtherBodyIndex :type Integer) (bFromSweep :type Boolean) (SweepResult :type "HitResult Structure (by ref)"))
  (bind _asbp_character (cast `/Game/Blueprints/BP_Character` OtherActor))
  (set `/Game/Blueprints/BP_Character.HasViola?` true _asbp_character)
  (`SceneComponent.SetVisibility` (`/Game/Blueprints/BP_Character.violin` _asbp_character) true false)
  (`self.K2_DestroyActor`)
  (`/Game/Blueprints/BP_Character.ViolaControls` _asbp_character)
  (`GameplayStatics.PlaySound2D` "/Game/Sounds/Violin_Pluck.Violin_Pluck" 1.0 1.0 0.0 null null))

(event `CustomEvent`
  (params (OverlappedComponent :type "PrimitiveComponent Object Reference") (OtherActor :type "Actor Object Reference") (OtherComp :type "PrimitiveComponent Object Reference") (OtherBodyIndex :type Integer) (bFromSweep :type Boolean) (SweepResult :type "HitResult Structure (by ref)"))
  (bind _asbp_character (cast `/Game/Blueprints/BP_Character` OtherActor))
  (set `/Game/Blueprints/BP_Character.Respawn Location` (`self.K2_GetActorLocation`) _asbp_character))

(event `self.ReceiveBeginPlay`
  (bind _returnvalue (`ActorComponent.GetOwner` (`self.violin`)))
  (bind (_returnvalue_x _returnvalue_y) (`KismetMathLibrary.BreakVector` (`self.K2_GetActorLocation` _returnvalue)))
  (`TimelineComponent.SetPlayRate` (`self.Timeline_0`) (/ 1.0 (`self.float_v`)))
  (bind (_direction _float_timing_viola) (`Timeline|Timeline_0`)
    (:`Update`
      (`self.K2_SetActorLocation` _returnvalue (`KismetMathLibrary.MakeVector` _returnvalue_x _returnvalue_y (`KismetMathLibrary.Lerp` (`self.TopPoint_v`) (`self.BottomPoint_v`) _float_timing_viola)) false false))))

(fn `UserConstructionScript`)