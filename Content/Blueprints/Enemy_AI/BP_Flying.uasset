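; BP_Flying is an enemy AI character with a flipbook sprite that moves along its facing direction and reverses at obstacles.
; MoveForward adds forward movement input, while wall detector overlap begins and ledge detector overlap ends both call TurnChar to rotate it 180 degrees.
; Helper functions, not called here, toggle dash speed and map movement states to player flipbooks, looping and left/right sprite rotation.
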(event `MoveForward`
  (`self.AddMovementInput` (`self.GetActorForwardVector`)))

(event `self.Walldetector.OnComponentBeginOverlap`
  (params (OverlappedComponent :type "PrimitiveComponent Object Reference") (OtherActor :type "Actor Object Reference") (OtherComp :type "PrimitiveComponent Object Reference") (OtherBodyIndex :type Integer) (bFromSweep :type Boolean) (SweepResult :type "HitResult Structure (by ref)"))
  (`self.TurnChar`))

(event `self.LedgeDetector.OnComponentEndOverlap`
  (params (OverlappedComponent :type "PrimitiveComponent Object Reference") (OtherActor :type "Actor Object Reference") (OtherComp :type "PrimitiveComponent Object Reference") (OtherBodyIndex :type Integer))
  (`self.TurnChar`))

(fn `F Set Movement States`
  (params (MovementStates :type "/Game/Blueprints/Enums/E_MovementStates Enum" :default "NewEnumerator0"))
  (bind _sprite (`self.Sprite`))
  (bind _sprite_2 (`self.Sprite`))
  (`PaperFlipbookComponent.SetLooping` (`self.Sprite`) (select `/Game/Blueprints/Enums/E_MovementStates` MovementStates :`NewEnumerator0` true :`NewEnumerator1` true :`NewEnumerator2` true :`NewEnumerator5` true :`NewEnumerator6` true))
  (`PaperFlipbookComponent.Play` (`self.Sprite`))
  (switch `/Game/Blueprints/Enums/E_MovementStates` MovementStates
    (:`NewEnumerator0`
      (`PaperFlipbookComponent.SetFlipbook` _sprite "/Game/SunnyLandAssets/sprites/player/idle/FB_player_idle.FB_player_idle"))
    (:`NewEnumerator1`
      (`PaperFlipbookComponent.SetFlipbook` _sprite "/Game/SunnyLandAssets/sprites/player/run/FB_player_run.FB_player_run")
      (`SceneComponent.K2_SetRelativeRotation` _sprite_2 (struct :`Yaw` -180.0) false false))
    (:`NewEnumerator2`
      (`PaperFlipbookComponent.SetFlipbook` _sprite "/Game/SunnyLandAssets/sprites/player/run/FB_player_run.FB_player_run")
      (`SceneComponent.K2_SetRelativeRotation` :`self` _sprite_2))
    (:`NewEnumerator5`
      (`PaperFlipbookComponent.SetFlipbook` _sprite "/Game/SunnyLandAssets/sprites/player/run/FB_player_dash.FB_player_dash")
      (`SceneComponent.K2_SetRelativeRotation` _sprite_2 (struct :`Yaw` -180.0) false false))
    (:`NewEnumerator6`
      (`PaperFlipbookComponent.SetFlipbook` _sprite "/Game/SunnyLandAssets/sprites/player/run/FB_player_dash.FB_player_dash")
      (`SceneComponent.K2_SetRelativeRotation` :`self` _sprite_2))
    (:`NewEnumerator3`
      (`PaperFlipbookComponent.SetFlipbook` _sprite "/Game/SunnyLandAssets/sprites/player/jump/FB_player_fall.FB_player_fall"))))

(fn `StartDash`
  (set `CharacterMovementComponent.MaxWalkSpeed` (`self.DashSpeed`) (`self.CharacterMovement`))
  (set `self.Dash` true))

(fn `StopDash`
  (set `CharacterMovementComponent.MaxWalkSpeed` (`self.WalkSpeed`) (`self.CharacterMovement`))
  (set `self.Dash` false))

(fn `TurnChar`
  (`self.K2_SetActorRotation` (`KismetMathLibrary.ComposeRotators` (`self.K2_GetActorRotation`) (struct :`Yaw` 180.0))))

(fn `UserConstructionScript`)