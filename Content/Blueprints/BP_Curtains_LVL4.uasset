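; BP_Curtains_LVL4 is a curtain actor that reacts to the player character and leads to a level change.
; Overlapping the box swaps the curtain sprite and spawns checkpoint particles, and leaving restores another sprite after a short delay.
; A separate teleport collision opens the LoadingScrn level after a delay.
; Construction sets translucent sort priority from world Y and places an arrow at TeleportLocation.
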(event `self.Box.OnComponentBeginOverlap`
  (params (OverlappedComponent :type "PrimitiveComponent Object Reference") (OtherActor :type "Actor Object Reference") (OtherComp :type "PrimitiveComponent Object Reference") (OtherBodyIndex :type Integer) (bFromSweep :type Boolean) (SweepResult :type "HitResult Structure (by ref)"))
  (bind _asbp_character (cast `/Game/Blueprints/BP_Character` OtherActor))
  (`PaperSpriteComponent.SetSprite` (`self.Curtains`) "/Game/sarah_assets/curtain/_v1_0000s_0004_5_Sprite._v1_0000s_0004_5_Sprite")
  (`NiagaraFunctionLibrary.SpawnSystemAtLocation` "/Game/Particle_Systems/Particles_Checkpoint.Particles_Checkpoint" (`self.K2_GetActorLocation`)))

(event `self.Box.OnComponentEndOverlap`
  (params (OverlappedComponent :type "PrimitiveComponent Object Reference") (OtherActor :type "Actor Object Reference") (OtherComp :type "PrimitiveComponent Object Reference") (OtherBodyIndex :type Integer))
  (cast `/Game/Blueprints/BP_Character` OtherActor)
  (`KismetSystemLibrary.Delay` 0.2)
  (`PaperSpriteComponent.SetSprite` (`self.Curtains`) "/Game/sarah_assets/curtain/_v1_0000s_0005_6_Sprite._v1_0000s_0005_6_Sprite"))

(event `self.teleport_collison.OnComponentBeginOverlap`
  (params (OverlappedComponent :type "PrimitiveComponent Object Reference") (OtherActor :type "Actor Object Reference") (OtherComp :type "PrimitiveComponent Object Reference") (OtherBodyIndex :type Integer) (bFromSweep :type Boolean) (SweepResult :type "HitResult Structure (by ref)"))
  (cast `/Game/Blueprints/BP_Character` OtherActor)
  (`KismetSystemLibrary.Delay` 2.0)
  (`GameplayStatics.OpenLevel` "LoadingScrn"))

(fn `UserConstructionScript`
  (bind _curtains (`self.Curtains`))
  (bind (_returnvalue_x _returnvalue_y) (`KismetMathLibrary.BreakVector` (`SceneComponent.K2_GetComponentLocation` _curtains)))
  (`PrimitiveComponent.SetTranslucentSortPriority` _curtains (`KismetMathLibrary.FTrunc` _returnvalue_y))
  (`SceneComponent.K2_SetRelativeTransform` (`self.Arrow`) (`self.teleportLocation`) false false))