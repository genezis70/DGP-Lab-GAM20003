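; BP_Block2 is a sprite block that BP_Violanote2 projectiles toggle on and off.
; An overlapping note is destroyed, and two FlipFlops alternate the sprite, then, after a short delay, the block's Y position and BlockState.
; A golem overlap forces the off state when the player character's AllowGolemAttack is true, without resetting either FlipFlop.
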(event `self.ReceiveBeginPlay`
  (bind _asbp_character (cast `/Game/Blueprints/BP_Character` (`GameplayStatics.GetPlayerCharacter` 0)))
  (set `self.Character ref` _asbp_character))

(event `self.BlockCol.OnComponentBeginOverlap`
  (params (OverlappedComponent :type "PrimitiveComponent Object Reference") (OtherActor :type "Actor Object Reference") (OtherComp :type "PrimitiveComponent Object Reference") (OtherBodyIndex :type Integer) (bFromSweep :type Boolean) (SweepResult :type "HitResult Structure (by ref)"))
  (bind (_returnvalue_x _returnvalue_y _returnvalue_z) (`KismetMathLibrary.BreakVector` (`self.K2_GetActorLocation`)))
  (bind (_returnvalue_x_2 _returnvalue_y_2 _returnvalue_z_2) (`KismetMathLibrary.BreakVector` (`self.K2_GetActorLocation`)))
  (bind _asbp_violanote_2 (cast `/Game/Blueprints/BP_Violanote2` OtherActor)
    (:`then`
      (`self.K2_DestroyActor` _asbp_violanote_2)
      (`/Engine/EditorBlueprintResources/StandardMacros.FlipFlop`
        (:`A`
          (`PaperSpriteComponent.SetSprite` (`self.Block`) "/Game/sarah_assets/v1_0004_flute-note_Sprite.v1_0004_flute-note_Sprite"))
        (:`B`
          (`PaperSpriteComponent.SetSprite` (`self.Block`) "/Game/sarah_assets/v1_0005_crochet_Sprite.v1_0005_crochet_Sprite")))
      (`KismetSystemLibrary.Delay` 0.2)
      (`/Engine/EditorBlueprintResources/StandardMacros.FlipFlop`
        (:`A`
          (`KismetSystemLibrary.PrintString` "on")
          (`self.K2_SetActorLocation` (`KismetMathLibrary.MakeVector` _returnvalue_x 0.0 _returnvalue_z))
          (set `self.Block State` true))
        (:`B`
          (`KismetSystemLibrary.PrintString` "off")
          (`self.K2_SetActorLocation` (`KismetMathLibrary.MakeVector` _returnvalue_x -25.0 _returnvalue_z))
          (set `self.Block State` false))))
    (:`CastFailed`
      (cast `/Game/Blueprints/Enemy_AI/AI_Ground/BP_Golem` OtherActor)
      (if (`/Game/Blueprints/BP_Character.Allow Golem Attack` (`self.Character ref`))
        (`PaperSpriteComponent.SetSprite` (`self.Block`) "/Game/sarah_assets/v1_0005_crochet_Sprite.v1_0005_crochet_Sprite")
        (`KismetSystemLibrary.PrintString` "off")
        (`self.K2_SetActorLocation` (`KismetMathLibrary.MakeVector` _returnvalue_x_2 -25.0 _returnvalue_z_2))
        (set `self.Block State` false)))))

(fn `UserConstructionScript`)