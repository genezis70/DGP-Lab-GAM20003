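; Flying 2D enemy character with events to move forward, chase the player or return to its spawn location.
; Chase and return use timeline-driven location lerps toward the target's X and Z, turning to face the travel direction.
; Wall and ledge detector overlaps set AI Blackboard flags and flip the actor 180 degrees.
; Helper functions switch player-named Paper2D flipbooks by movement state and toggle dash speed.
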(event `MoveForward`
  ;[1 1 1] Move Forward
  (`self.AddMovementInput` (`self.GetActorForwardVector`)))

(event `Track`
  (bind (_returnvalue_x _returnvalue_y _returnvalue_z) (`KismetMathLibrary.BreakVector` (`self.K2_GetActorLocation`)))
  (bind _returnvalue_x_2 (`KismetMathLibrary.BreakVector` (`self.K2_GetActorLocation`)))
  ;[1 1 1] Track Player
  (bind _asbp_character (cast `/Game/Blueprints/BP_Character` (`GameplayStatics.GetPlayerCharacter` 0)))
  (bind (_direction _walky) (`Timeline|Timeline` :!via `PlayFromStart`)
    (:`Update`
      (`self.K2_SetActorLocation` (`KismetMathLibrary.VLerp` (`KismetMathLibrary.MakeVector` _returnvalue_x _returnvalue_y _returnvalue_z) (`KismetMathLibrary.MakeVector` (.x (`self.K2_GetActorLocation` _asbp_character)) 0.0 (.z (`self.K2_GetActorLocation` _asbp_character))) _walky))
      (bind _returnvalue_x_3 (`KismetMathLibrary.BreakVector` (`self.K2_GetActorLocation` _asbp_character)))
      (if (> _returnvalue_x_3 _returnvalue_x_2)
        (`self.K2_SetActorRotation` (struct))
        (else
          (`self.K2_SetActorRotation` (struct :`Yaw` 180.0)))))))

(event `self.Walldetector.OnComponentBeginOverlap`
  (params (OverlappedComponent :type "PrimitiveComponent Object Reference") (OtherActor :type "Actor Object Reference") (OtherComp :type "PrimitiveComponent Object Reference") (OtherBodyIndex :type Integer) (bFromSweep :type Boolean) (SweepResult :type "HitResult Structure (by ref)"))
  ;[1 1 1] Wall Detector
  (`BlackboardComponent.SetValueAsBool` (`AIBlueprintHelperLibrary.GetBlackboard` (`AIBlueprintHelperLibrary.GetAIController` self)) "Walldetection" true)
  (`self.TurnChar`))

(event `self.Walldetector.OnComponentEndOverlap`
  (params (OverlappedComponent :type "PrimitiveComponent Object Reference") (OtherActor :type "Actor Object Reference") (OtherComp :type "PrimitiveComponent Object Reference") (OtherBodyIndex :type Integer))
  ;[1 1 1] Wall Detector
  (`BlackboardComponent.SetValueAsBool` (`AIBlueprintHelperLibrary.GetBlackboard` (`AIBlueprintHelperLibrary.GetAIController` self)) "Walldetection" false))

(event `Go to Start`
  (bind (_returnvalue_x _returnvalue_y _returnvalue_z) (`KismetMathLibrary.BreakVector` (`self.K2_GetActorLocation`)))
  (bind _returnvalue_x_2 (`KismetMathLibrary.BreakVector` (`self.K2_GetActorLocation`)))
  (bind _start_x (`KismetMathLibrary.BreakVector` (`self.Start`)))
  ;[1 1 1] Go to Start
  (bind (_direction _walky) (`Timeline|Timeline_0` :!via `PlayFromStart`)
    (:`Update`
      (`self.K2_SetActorLocation` (`KismetMathLibrary.VLerp` (`KismetMathLibrary.MakeVector` _returnvalue_x _returnvalue_y _returnvalue_z) (`KismetMathLibrary.MakeVector` (.x (`self.Start`)) 0.0 (.z (`self.Start`))) _walky))
      (if (> _returnvalue_x_2 _start_x)
        (`self.K2_SetActorRotation` (struct :`Yaw` 180.0))
        (else
          (`self.K2_SetActorRotation` (struct)))))))

(event `self.LedgeDetector.OnComponentEndOverlap`
  (params (OverlappedComponent :type "PrimitiveComponent Object Reference") (OtherActor :type "Actor Object Reference") (OtherComp :type "PrimitiveComponent Object Reference") (OtherBodyIndex :type Integer))
  ;[1 1 1] Ledge Detector
  (`BlackboardComponent.SetValueAsBool` (`AIBlueprintHelperLibrary.GetBlackboard` (`AIBlueprintHelperLibrary.GetAIController` self)) "Ledgedetection" true)
  (`self.TurnChar`))

(event `self.ReceiveBeginPlay`
  ;[1 1 1] Set Start Location
  (bind _output_get (set `self.Start` (`self.K2_GetActorLocation`)))
  (`KismetSystemLibrary.PrintString` (`KismetStringLibrary.Conv_VectorToString` _output_get)))

(fn `F Set Movement States`
  (params (MovementStates :type "/Game/Blueprints/Enums/E_MovementStates Enum" :default "NewEnumerator0"))
  (bind _sprite (`self.Sprite`))
  (bind _sprite_2 (`self.Sprite`))
  (`PaperFlipbookComponent.SetLooping` (`self.Sprite`) (select `/Game/Blueprints/Enums/E_MovementStates` MovementStates :`NewEnumerator0` true :`NewEnumerator1` true :`NewEnumerator2` true :`NewEnumerator5` true :`NewEnumerator6` true))
  (`PaperFlipbookComponent.Play` (`self.Sprite`))
  (switch `/Game/Blueprints/Enums/E_MovementStates` MovementStates
    (:`NewEnumerator0`
      (`PaperFlipbookComponent.SetFlipbook` _sprite "/Game/SunnyLandAssets/sprites/player/idle/FB_player_idle.FB_player_idle"))
    (:`NewEnumerator1`
      (`PaperFlipbookComponent.SetFlipbook` _sprite "/Game/SunnyLandAssets/sprites/player/run/FB_player_run.FB_player_run")
      (`SceneComponent.K2_SetRelativeRotation` _sprite_2 (struct :`Yaw` -180.0) false false))
    (:`NewEnumerator2`
      (`PaperFlipbookComponent.SetFlipbook` _sprite "/Game/SunnyLandAssets/sprites/player/run/FB_player_run.FB_player_run")
      (`SceneComponent.K2_SetRelativeRotation` :`self` _sprite_2))
    (:`NewEnumerator5`
      (`PaperFlipbookComponent.SetFlipbook` _sprite "/Game/SunnyLandAssets/sprites/player/run/FB_player_dash.FB_player_dash")
      (`SceneComponent.K2_SetRelativeRotation` _sprite_2 (struct :`Yaw` -180.0) false false))
    (:`NewEnumerator6`
      (`PaperFlipbookComponent.SetFlipbook` _sprite "/Game/SunnyLandAssets/sprites/player/run/FB_player_dash.FB_player_dash")
      (`SceneComponent.K2_SetRelativeRotation` :`self` _sprite_2))
    (:`NewEnumerator3`
      (`PaperFlipbookComponent.SetFlipbook` _sprite "/Game/SunnyLandAssets/sprites/player/jump/FB_player_fall.FB_player_fall"))))

(fn `StartDash`
  (set `CharacterMovementComponent.MaxWalkSpeed` (`self.DashSpeed`) (`self.CharacterMovement`))
  (set `self.Dash` true))

(fn `StopDash`
  (set `CharacterMovementComponent.MaxWalkSpeed` (`self.WalkSpeed`) (`self.CharacterMovement`))
  (set `self.Dash` false))

(fn `TurnChar`
  (`self.K2_SetActorRotation` (`KismetMathLibrary.ComposeRotators` (`self.K2_GetActorRotation`) (struct :`Yaw` 180.0))))

(fn `UserConstructionScript`)