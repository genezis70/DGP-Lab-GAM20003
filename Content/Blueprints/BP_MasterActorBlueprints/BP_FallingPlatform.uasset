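; BP_FallingPlatform is a sprite platform that drops after the player touches it and later respawns.
; The first Box overlap by PlayerCharacterRef waits DropDelay, adds an active ProjectileMovement component and switches the sprite's collision object type to PhysicsBody.
; After RespawnPlatformDelay it spawns a fresh copy at the location saved on BeginPlay; this graph never destroys the fallen one.
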(event `self.ReceiveBeginPlay`
  (`parent.ReceiveBeginPlay`)
  (set `self.StartingLocationplatform` (`self.K2_GetActorLocation`)))

(event `self.Box.OnComponentBeginOverlap`
  (params (OverlappedComponent :type "PrimitiveComponent Object Reference") (OtherActor :type "Actor Object Reference") (OtherComp :type "PrimitiveComponent Object Reference") (OtherBodyIndex :type Integer) (bFromSweep :type Boolean) (SweepResult :type "HitResult Structure (by ref)"))
  (if (== OtherActor (`self.PlayerCharacterRef`))
    (`/Engine/EditorBlueprintResources/StandardMacros.DoOnce` false
      (:`Completed`
        (`KismetSystemLibrary.Delay` (`self.dropDelay`))
        (bind _returnvalue (`AddComponent|NODE_AddProjectileMovementComponent-0` :`self` self))
        (`ActorComponent.SetActive` _returnvalue true false)
        (`PrimitiveComponent.SetCollisionObjectType` (`self.PaperSprite`) "ECC_PhysicsBody")
        (`KismetSystemLibrary.Delay` (`self.RespawnPlatformDelay`))
        (`|SpawnActorFromClass` "BP_FallingPlatform_C" (`KismetMathLibrary.Conv_VectorToTransform` (`self.StartingLocationplatform`)) "Undefined" "MultiplyWithRoot" null null)))))

(fn `UserConstructionScript`
  (`parent.UserConstructionScript`))