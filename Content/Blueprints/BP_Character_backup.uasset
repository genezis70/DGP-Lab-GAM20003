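; Paper2D player character with Enhanced Input movement, jump, timed dash, baton attack and a hold-to-show instrument menu.
; Input events pick flipbook and facing through FSetMovementStates, with a looping timer restoring idle after landing.
; Dash and attack read Dash and Launch flags, apparently meant for beat timing; sphere-trace hits launch BP_Ground characters, harder on crits.
; Trigger box overlaps toggle PlayerTrigger, and Tick flushes debug lines.
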(event `self.ReceiveBeginPlay`
  ;[0.3451 0.7843 1] Initial Mapping Context
  (bind _aspc_character (cast `/Game/Blueprints/PC_Character` (`GameplayStatics.GetPlayerController` 0)))
  (`/Engine/EditorBlueprintResources/StandardMacros.IsValid` _aspc_character
    (:`Is Valid`
      (bind _returnvalue (pcsubsystem `EnhancedInputLocalPlayerSubsystem` _aspc_character))
      (`/Engine/EditorBlueprintResources/StandardMacros.IsValid` _returnvalue
        (:`Is Valid`
          (`EnhancedInputSubsystemInterface.AddMappingContext` _returnvalue "/Game/Blueprints/Input/IMC_Baton.IMC_Baton" 0 (struct))
          ;[0.8392 0.3647 1] Hiding Instrument Menu at the start of the game
          (bind _returnvalue_2 (`|CreateWidget` "/Game/Blueprints/UI/UI_Instruments.UI_Instruments_C" (`GameplayStatics.GetPlayerController` 0)))
          (bind _output_get (set `self.UIInstrumentRef` _returnvalue_2))
          (`UserWidget.AddToViewport` _output_get 0)
          (`Widget.SetVisibility` (`self.UIInstrumentRef`) "Hidden"))))))

(event `EnhancedInput|/Game/Blueprints/Input/IA_Movement`
  (params (ActionValue :type "Float (double-precision)") (ElapsedSeconds :type "Float (double-precision)") (TriggeredSeconds :type "Float (double-precision)") (InputAction :type "InputAction Object Reference" :default "/Game/Blueprints/Input/IA_Movement.IA_Movement"))
  ;[0.3451 0.7843 1] Basic Run and Dash Movement
  (:`Triggered`
    (set `self.MovementActionValue` ActionValue)
    (`self.AddMovementInput` (`self.GetActorForwardVector`) ActionValue)
    (if (`NavMovementComponent.IsFalling` (`self.CharacterMovement`))
      (`self.F Set Movement States` "NewEnumerator3")
      (`self.CheckIsFalling`)
      (elif (> ActionValue 0.0)
        (if (`self.Dash`)
          (`self.F Set Movement States` "NewEnumerator6")
          (else
            (`self.F Set Movement States` "NewEnumerator2")))
        (elif (< ActionValue 0.0)
          (if (`self.Dash`)
            (`self.F Set Movement States` "NewEnumerator5")
            (else
              (`self.F Set Movement States` "NewEnumerator1")))
          (else
            (`self.F Set Movement States` "NewEnumerator0"))))))
  (:`Completed`
    (set `self.MovementActionValue` 0.0)
    (if (not (`NavMovementComponent.IsFalling` (`self.CharacterMovement`)))
      (`self.F Set Movement States` "NewEnumerator0"))))

(event `EnhancedInput|/Game/Blueprints/Input/IA_Jump`
  (params (ActionValue :type Boolean) (ElapsedSeconds :type "Float (double-precision)") (TriggeredSeconds :type "Float (double-precision)") (InputAction :type "InputAction Object Reference" :default "/Game/Blueprints/Input/IA_Jump.IA_Jump"))
  ;[0.3451 0.7843 1] Jump Movement
  (:`Triggered`
    (`self.Jump`)
    (`self.F Set Movement States` "NewEnumerator3")
    (`self.CheckIsFalling`)))

(event `CheckIsFalling`
  ;[1 0.2344 0.2344] Checks if Player is falling
  (bind _returnvalue (`KismetSystemLibrary.K2_SetTimerDelegate` (delegate `CheckIsFallingLoop`) 0.05 true))
  (set `self.CheckIsFallingTimerHandle` _returnvalue))

(event `CheckIsFallingLoop`
  ;[1 0.2344 0.2344] Checks if Player is falling
  (if (not (`NavMovementComponent.IsFalling` (`self.CharacterMovement`)))
    (`KismetSystemLibrary.K2_ClearAndInvalidateTimerHandle` (`self.CheckIsFallingTimerHandle`))
    (if (== (`self.MovementActionValue`) 0.0)
      (`self.F Set Movement States` "NewEnumerator0"))))

(event `self.ReceiveTick`
  (params (DeltaSeconds :type "Float (single-precision)"))
  ;[1 1 1] Remove Sphere Trace
  (`KismetSystemLibrary.FlushPersistentDebugLines`))

(event `EnhancedInput|/Game/Blueprints/Input/IA_Special_Dash`
  (params (ActionValue :type Boolean) (ElapsedSeconds :type "Float (double-precision)") (TriggeredSeconds :type "Float (double-precision)") (InputAction :type "InputAction Object Reference" :default "/Game/Blueprints/Input/IA_Special_Dash.IA_Special_Dash"))
  ;[0.3451 0.7843 1] Allows Dash Movement at Beat 1
  (:`Triggered`
    (if (`self.Dash`)
      (`self.StartDash`)
      (`KismetSystemLibrary.Delay` 0.5)
      (`self.StopDash`))))

(event `EnhancedInput|/Game/Blueprints/Input/IA_InstrumentMenu`
  (params (ActionValue :type Boolean) (ElapsedSeconds :type "Float (double-precision)") (TriggeredSeconds :type "Float (double-precision)") (InputAction :type "InputAction Object Reference" :default "/Game/Blueprints/Input/IA_InstrumentMenu.IA_InstrumentMenu"))
  ;[0.8392 0.3647 1] Shows and Hides Instrument Menu with Right Click
  (:`Triggered`
    (`Widget.SetVisibility` (`self.UIInstrumentRef`) "Visible"))
  (:`Completed`
    (`Widget.SetVisibility` (`self.UIInstrumentRef`) "Hidden")))

(event `self.ReceiveActorBeginOverlap`
  (params (OtherActor :type "Actor Object Reference"))
  ;[1 0.706 0] Trigger Box (Flying)
  (cast `TriggerBox` OtherActor)
  (`KismetSystemLibrary.PrintString` "Hello")
  (set `self.Player_Trigger` true))

(event `EnhancedInput|/Game/Blueprints/Input/IA_Baton_Attack`
  (params (ActionValue :type Boolean) (ElapsedSeconds :type "Float (double-precision)") (TriggeredSeconds :type "Float (double-precision)") (InputAction :type "InputAction Object Reference" :default "/Game/Blueprints/Input/IA_Baton_Attack.IA_Baton_Attack"))
  (bind _returnvalue (`self.K2_GetActorLocation` self))
  (bind _returnvalue_2 (`self.K2_GetActorLocation` self))
  ;[1 1 1] Baton Attack
  (:`Triggered`
    (if (`self.Launch`)
      ;[1 1 1] Critical Hit
      (bind (_outhit _returnvalue_3) (`KismetSystemLibrary.SphereTraceSingleForObjects` _returnvalue (+ _returnvalue (* (`self.GetActorForwardVector` self) 1.0)) 10.0 (`|MakeArray` "ObjectTypeQuery3" :!type "EObjectTypeQuery Enum")))
      (if _returnvalue_3
        (bind _asbp_ground (cast `/Game/Blueprints/Enemy_AI/AI_Ground/BP_Ground` (`.HitActor` (`GameplayStatics.BreakHitResult` _outhit))))
        (`self.LaunchCharacter` _asbp_ground (300.0 0.0 300.0) false false)
        (`KismetSystemLibrary.PrintString` "Crit!!"))
      (else
        ;[1 1 1] Regular Hit
        (bind (_outhit_2 _returnvalue_4) (`KismetSystemLibrary.SphereTraceSingleForObjects` :`Start` _returnvalue_2 :`End` (+ _returnvalue_2 (* (`self.GetActorForwardVector` self) 1.0)) :`Radius` 10.0 :`ObjectTypes` (`|MakeArray` "ObjectTypeQuery3" :!type "EObjectTypeQuery Enum") :`DrawDebugType` "ForDuration"))
        (if _returnvalue_4
          (bind _asbp_ground_2 (cast `/Game/Blueprints/Enemy_AI/AI_Ground/BP_Ground` (`.HitActor` (`GameplayStatics.BreakHitResult` _outhit_2))))
          (`self.LaunchCharacter` _asbp_ground_2 (200.0 0.0 100.0) false false))))))

(event `self.ReceiveActorEndOverlap`
  (params (OtherActor :type "Actor Object Reference"))
  ;[1 0.706 0] Trigger Box (Flying)
  (cast `TriggerBox` OtherActor)
  (`KismetSystemLibrary.PrintString` "Cya Loser")
  (set `self.Player_Trigger` false))

(fn `F Set Movement States`
  (params (MovementStates :type "/Game/Blueprints/Enums/E_MovementStates Enum" :default "NewEnumerator0"))
  (bind _sprite (`self.Sprite`))
  (bind _sprite_2 (`self.Sprite`))
  (`PaperFlipbookComponent.SetLooping` (`self.Sprite`) (select `/Game/Blueprints/Enums/E_MovementStates` MovementStates :`NewEnumerator0` true :`NewEnumerator1` true :`NewEnumerator2` true :`NewEnumerator5` true :`NewEnumerator6` true))
  (`PaperFlipbookComponent.Play` (`self.Sprite`))
  (switch `/Game/Blueprints/Enums/E_MovementStates` MovementStates
    (:`NewEnumerator0`
      (`PaperFlipbookComponent.SetFlipbook` _sprite "/Game/SunnyLandAssets/sprites/player/idle/FB_player_idle.FB_player_idle"))
    (:`NewEnumerator1`
      (`PaperFlipbookComponent.SetFlipbook` _sprite "/Game/SunnyLandAssets/sprites/player/run/FB_player_run.FB_player_run")
      (`SceneComponent.K2_SetRelativeRotation` _sprite_2 (struct :`Yaw` -180.0) false false))
    (:`NewEnumerator2`
      (`PaperFlipbookComponent.SetFlipbook` _sprite "/Game/SunnyLandAssets/sprites/player/run/FB_player_run.FB_player_run")
      (`SceneComponent.K2_SetRelativeRotation` :`self` _sprite_2))
    (:`NewEnumerator5`
      (`PaperFlipbookComponent.SetFlipbook` _sprite "/Game/SunnyLandAssets/sprites/player/run/FB_player_dash.FB_player_dash")
      (`SceneComponent.K2_SetRelativeRotation` _sprite_2 (struct :`Yaw` -180.0) false false))
    (:`NewEnumerator6`
      (`PaperFlipbookComponent.SetFlipbook` _sprite "/Game/SunnyLandAssets/sprites/player/run/FB_player_dash.FB_player_dash")
      (`SceneComponent.K2_SetRelativeRotation` :`self` _sprite_2))
    (:`NewEnumerator3`
      (`PaperFlipbookComponent.SetFlipbook` _sprite "/Game/SunnyLandAssets/sprites/player/jump/FB_player_fall.FB_player_fall"))))

(fn `StartDash`
  (set `CharacterMovementComponent.MaxWalkSpeed` (`self.DashSpeed`) (`self.CharacterMovement`))
  (set `self.Dash` true))

(fn `StopDash`
  (set `CharacterMovementComponent.MaxWalkSpeed` (`self.WalkSpeed`) (`self.CharacterMovement`))
  (set `self.Dash` false))

(fn `UserConstructionScript`)