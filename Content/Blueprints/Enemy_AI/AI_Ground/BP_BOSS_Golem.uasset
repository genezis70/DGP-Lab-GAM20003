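; Golem boss enemy, a 2D flipbook character that walks or halts according to the player character's beat flag and turns at walls and ledges.
; Its attack, gated by another player flag, sphere-traces to damage and launch the player, or destroy a slime.
; Violin notes damage and knock it back until it dies, with health polled each Tick into a widget bar.
; Movement-state and dash functions reference player flipbooks and go uncalled here.
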(event `self.ReceiveBeginPlay`
  ;[1 1 1] Event begin play
  (set `self.GolemLives` 4.0))

(event `StopAI`
  ;[1 1 1] Stop AI From Moving
  (`self.AddMovementInput` (`self.GetActorForwardVector`) 0.0 true)
  (`PaperFlipbookComponent.SetFlipbook` (`self.Sprite`) "/Game/KaI_Assets/golem/golem_MOVE1.golem_MOVE1"))

(event `MoveForward`
  ;[1 1 1] Make AI Move
  (`self.AddMovementInput` (`self.GetActorForwardVector`))
  (`PaperFlipbookComponent.SetFlipbook` (`self.Sprite`) "/Game/KaI_Assets/golem/golem_MOVE1.golem_MOVE1"))

(event `self.Walldetector.OnComponentBeginOverlap`
  (params (OverlappedComponent :type "PrimitiveComponent Object Reference") (OtherActor :type "Actor Object Reference") (OtherComp :type "PrimitiveComponent Object Reference") (OtherBodyIndex :type Integer) (bFromSweep :type Boolean) (SweepResult :type "HitResult Structure (by ref)"))
  ;[1 1 1] Detects Walls and Turns AI
  (if (`self.ActorHasTag` OtherActor "Block")
    (`self.TurnChar`)
    (`KismetSystemLibrary.PrintString` "Hello")))

(event `Tell AI To Move`
  ;[1 1 1] Move At Beat 1
  (bind _asbp_character (cast `/Game/Blueprints/BP_Character` (`GameplayStatics.GetPlayerCharacter` 0)))
  (if (`/Game/Blueprints/BP_Character.TellAIToMove` _asbp_character)
    (`self.MoveForward`)
    (else
      (`self.StopAI`))))

(event `self.ReceiveAnyDamage`
  (params (Damage :type "Float (single-precision)") (DamageType :type "DamageType Object Reference") (InstigatedBy :type "Controller Object Reference") (DamageCauser :type "Actor Object Reference"))
  ;[1 1 1] Damage
  (bind _output_get (set `self.GolemLives` (`KismetMathLibrary.FClamp` (- (`self.GolemLives`) Damage) 0.0 (`self.GolemLivesMax`))))
  (if (== _output_get 0.0)
    (`self.K2_DestroyActor`)))

(event `self.LedgeDetector.OnComponentEndOverlap`
  (params (OverlappedComponent :type "PrimitiveComponent Object Reference") (OtherActor :type "Actor Object Reference") (OtherComp :type "PrimitiveComponent Object Reference") (OtherBodyIndex :type Integer))
  ;[1 1 1] Detects Ledges and Turns AI
  (`self.TurnChar`))

(event `update health`)

(event `self.ReceiveTick`
  (params (DeltaSeconds :type "Float (single-precision)"))
  (bind _asai_healthbar (cast `/Game/Blueprints/Enemy_AI/AI_Ground/AI_Healthbar` (`WidgetComponent.GetWidget` (`self.Health`))))
  (`ProgressBar.SetPercent` (`/Game/Blueprints/Enemy_AI/AI_Ground/AI_Healthbar.Healthbar` _asai_healthbar) (/ (`self.GolemLives`) 4.0))
  (`Widget.SetVisibility` _asai_healthbar "Visible"))

(event `self.Back.OnComponentBeginOverlap`
  (params (OverlappedComponent :type "PrimitiveComponent Object Reference") (OtherActor :type "Actor Object Reference") (OtherComp :type "PrimitiveComponent Object Reference") (OtherBodyIndex :type Integer) (bFromSweep :type Boolean) (SweepResult :type "HitResult Structure (by ref)"))
  ;[1 1 1] Detects if player is behind them and turns AI
  (bind _asbp_character (cast `/Game/Blueprints/BP_Character` OtherActor))
  (`self.AddMovementInput` (`self.GetActorForwardVector` _asbp_character))
  (`self.K2_SetActorRotation` (struct :`Yaw` 180.0)))

(event `Attack`
  (bind _returnvalue_x (`KismetMathLibrary.BreakVector` (`self.K2_GetActorLocation`)))
  (bind _returnvalue (`self.K2_GetActorLocation` self))
  ;[1 1 1] Attack Player
  (bind _asbp_character (cast `/Game/Blueprints/BP_Character` (`GameplayStatics.GetPlayerCharacter` 0)))
  (if (`/Game/Blueprints/BP_Character.Allow Golem Attack` _asbp_character)
    (bind (_outhit _returnvalue_2) (`KismetSystemLibrary.SphereTraceSingleForObjects` :`Start` _returnvalue :`End` (+ _returnvalue (* (`self.GetActorForwardVector` self) 1.0)) :`Radius` 50.0 :`ObjectTypes` (`|MakeArray` "ObjectTypeQuery3" :!type "EObjectTypeQuery Enum") :`DrawDebugType` "ForDuration"))
    (if _returnvalue_2
      (bind (_bblockinghit _binitialoverlap _time _distance _location _impactpoint _normal _impactnormal _physmat _hitactor) (`GameplayStatics.BreakHitResult` _outhit))
      (bind _asbp_character_2 (cast `/Game/Blueprints/BP_Character` _hitactor)
        (:`then`
          (bind _returnvalue_x_2 (`KismetMathLibrary.BreakVector` (`self.K2_GetActorLocation` _asbp_character_2)))
          (if (> _returnvalue_x _returnvalue_x_2)
            (`self.LaunchCharacter` _asbp_character_2 (-300.0 0.0 200.0) false false)
            (else
              (`self.LaunchCharacter` _asbp_character_2 (300.0 0.0 200.0) false false)))
          (bind _returnvalue_3 (`GameplayStatics.ApplyDamage` _asbp_character_2 50.0 null self))
          (`KismetSystemLibrary.PrintString` (`KismetStringLibrary.Conv_DoubleToString` _returnvalue_3))
          (`GameplayStatics.PlaySound2D` "/Game/Sounds/enemy_hit.enemy_hit" 1.0 1.0 0.0 null null))
        (:`CastFailed`
          (bind _asbp_slime (cast `/Game/Blueprints/Enemy_AI/AI_Ground/Slime/BP_Slime` _hitactor))
          (`self.K2_DestroyActor` _asbp_slime))))))

(event `self.Front.OnComponentBeginOverlap`
  (params (OverlappedComponent :type "PrimitiveComponent Object Reference") (OtherActor :type "Actor Object Reference") (OtherComp :type "PrimitiveComponent Object Reference") (OtherBodyIndex :type Integer) (bFromSweep :type Boolean) (SweepResult :type "HitResult Structure (by ref)"))
  ;[1 1 1] Knockback
  (cast `/Game/Blueprints/BP_Character` OtherActor)
  (set `self.Knockback` true))

(event `self.Front.OnComponentEndOverlap`
  (params (OverlappedComponent :type "PrimitiveComponent Object Reference") (OtherActor :type "Actor Object Reference") (OtherComp :type "PrimitiveComponent Object Reference") (OtherBodyIndex :type Integer))
  ;[1 1 1] Knockback
  (cast `/Game/Blueprints/BP_Character` OtherActor)
  (set `self.Knockback` false))

(event `self.CapsuleComponent.OnComponentBeginOverlap`
  (params (OverlappedComponent :type "PrimitiveComponent Object Reference") (OtherActor :type "Actor Object Reference") (OtherComp :type "PrimitiveComponent Object Reference") (OtherBodyIndex :type Integer) (bFromSweep :type Boolean) (SweepResult :type "HitResult Structure (by ref)"))
  (bind _returnvalue_x (`KismetMathLibrary.BreakVector` (`self.GetActorForwardVector` (`GameplayStatics.GetPlayerCharacter` 0))))
  ;[1 1 1] Damage
  (bind _asbp_violin_note_2 (cast `/Game/Blueprints/BP_Violin_Note2` OtherActor))
  (`GameplayStatics.ApplyDamage` self 1.0)
  (`self.LaunchCharacter` (`KismetMathLibrary.MakeVector` (* _returnvalue_x 100.0) 0.0 100.0))
  (`GameplayStatics.PlaySound2D` "/Game/Sounds/enemy_hit.enemy_hit" 1.0 1.0 0.0 null null)
  (`self.K2_DestroyActor` _asbp_violin_note_2))

(fn `F Set Movement States`
  (params (MovementStates :type "/Game/Blueprints/Enums/E_MovementStates Enum" :default "NewEnumerator0"))
  (bind _sprite (`self.Sprite`))
  (bind _sprite_2 (`self.Sprite`))
  (`PaperFlipbookComponent.SetLooping` (`self.Sprite`) (select `/Game/Blueprints/Enums/E_MovementStates` MovementStates :`NewEnumerator0` true :`NewEnumerator1` true :`NewEnumerator2` true :`NewEnumerator5` true :`NewEnumerator6` true))
  (`PaperFlipbookComponent.Play` (`self.Sprite`))
  (switch `/Game/Blueprints/Enums/E_MovementStates` MovementStates
    (:`NewEnumerator0`
      (`PaperFlipbookComponent.SetFlipbook` _sprite "/Game/SunnyLandAssets/sprites/player/idle/FB_player_idle.FB_player_idle"))
    (:`NewEnumerator1`
      (`PaperFlipbookComponent.SetFlipbook` _sprite "/Game/SunnyLandAssets/sprites/player/run/FB_player_run.FB_player_run")
      (`SceneComponent.K2_SetRelativeRotation` _sprite_2 (struct :`Yaw` -180.0) false false))
    (:`NewEnumerator2`
      (`PaperFlipbookComponent.SetFlipbook` _sprite "/Game/SunnyLandAssets/sprites/player/run/FB_player_run.FB_player_run")
      (`SceneComponent.K2_SetRelativeRotation` :`self` _sprite_2))
    (:`NewEnumerator5`
      (`PaperFlipbookComponent.SetFlipbook` _sprite "/Game/SunnyLandAssets/sprites/player/run/FB_player_dash.FB_player_dash")
      (`SceneComponent.K2_SetRelativeRotation` _sprite_2 (struct :`Yaw` -180.0) false false))
    (:`NewEnumerator6`
      (`PaperFlipbookComponent.SetFlipbook` _sprite "/Game/SunnyLandAssets/sprites/player/run/FB_player_dash.FB_player_dash")
      (`SceneComponent.K2_SetRelativeRotation` :`self` _sprite_2))
    (:`NewEnumerator3`
      (`PaperFlipbookComponent.SetFlipbook` _sprite "/Game/SunnyLandAssets/sprites/player/jump/FB_player_fall.FB_player_fall"))))

(fn `StartDash`
  (set `CharacterMovementComponent.MaxWalkSpeed` (`self.DashSpeed`) (`self.CharacterMovement`))
  (set `self.Dash` true))

(fn `StopDash`
  (set `CharacterMovementComponent.MaxWalkSpeed` (`self.WalkSpeed`) (`self.CharacterMovement`))
  (set `self.Dash` false))

(fn `TurnChar`
  (`self.K2_SetActorRotation` (`KismetMathLibrary.ComposeRotators` (`self.K2_GetActorRotation`) (struct :`Yaw` 180.0))))

(fn `UserConstructionScript`)