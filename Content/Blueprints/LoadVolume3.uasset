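; Level 3 load volume that resets the overlapping player's stats, updates or creates the save slot and starts the level's beat-driven gameplay.
; It adds a metronome widget, starts layered music with sound mixes, and creates 108 BPM Quartz player and AI clocks, the latter name requested twice.
; Beat callbacks toggle character flags on beat one to gate golem and slime attacks, AI movement, dash, launch and shooting.
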(event `self.ReceiveTick`
  (params (DeltaSeconds :type "Float (single-precision)")))

(event `self.ReceiveActorBeginOverlap`
  (params (OtherActor :type "Actor Object Reference"))
  (bind _asbp_character (cast `/Game/Blueprints/BP_Character` OtherActor))
  (set `/Game/Blueprints/BP_Character.HP` (`/Game/Blueprints/BP_Character.Max HP` _asbp_character) _asbp_character)
  (set `/Game/Blueprints/BP_Character.Lives` (`/Game/Blueprints/BP_Character.Total Lives` _asbp_character) _asbp_character)
  (set `/Game/Blueprints/BP_Character.SheetmusicCollected` 0.0 _asbp_character)
  (`|CreateWidget` "/Game/Blueprints/UI/Metronome.Metronome_C")
  (`KismetSystemLibrary.PrintString` "load")
  (set `/Game/Blueprints/BP_Character.Load` true _asbp_character)
  (bind _returnvalue (`GameplayStatics.DoesSaveGameExist` "save1"))
  (if _returnvalue
    (bind _returnvalue_2 (`GameplayStatics.LoadGameFromSlot` "save1"))
    (bind _asbp_level_save (cast `/Game/Blueprints/BP_LevelSave` _returnvalue_2))
    (bind _output_get (set `/Game/Blueprints/BP_LevelSave.Level Name` "Level3" _asbp_level_save))
    (`KismetSystemLibrary.PrintString` (`KismetStringLibrary.Conv_NameToString` _output_get))
    (`GameplayStatics.SaveGameToSlot` _asbp_level_save "save1")
    (else
      (bind _returnvalue_3 (`GameplayStatics.CreateSaveGameObject` "/Game/Blueprints/BP_LevelSave.BP_LevelSave_C"))
      (`GameplayStatics.SaveGameToSlot` _returnvalue_3 "save1")))
  ;[1 1 1] Create Player Clock
  (`KismetSystemLibrary.PrintString` "GAME SAVED")
  (bind _asbp_character_2 (cast `/Game/Blueprints/BP_Character` (`GameplayStatics.GetPlayerCharacter` 0)))
  (bind _output_get_2 (set `self.As BP Character` _asbp_character_2))
  (set `/Game/Blueprints/BP_Character.allowwalkingsound` true _output_get_2)
  (bind _returnvalue_4 (`|CreateWidget` "/Game/Blueprints/UI/Metronome.Metronome_C"))
  (`UserWidget.AddToViewport` _returnvalue_4 0)
  (bind _returnvalue_5 (`QuartzSubsystem.CreateNewClock` (subsystem `QuartzSubsystem`) "MetronomePlayer" (make `QuartzClockSettings` (make `QuartzTimeSignature` 4)) false true))
  (bind _clockhandle (`QuartzClockHandle.SetBeatsPerMinute` :`self` _returnvalue_5 :`BeatsPerMinute` 108.0))
  (bind _output_get_3 (set `self.Metronome108` _clockhandle))
  ;[1 1 1] Start Player Clock
  (`QuartzClockHandle.StartClock` _output_get_3)
  (`QuartzClockHandle.SubscribeToQuantizationEvent` (`self.Metronome108`) "Beat" (delegate `Beats`))
  ;[1 1 1] Spawn Forest Theme
  (`GameplayStatics.PlaySound2D` "/Game/Music/Level_2_Loop.Level_2_Loop" 1.0 1.0 0.0 null (`self.As BP Character`))
  (`GameplayStatics.SetBaseSoundMix` "/Game/Music/Mixes/UnmuteMusic3.UnmuteMusic3")
  (`GameplayStatics.PlaySound2D` "/Game/Music/Deep_Treble_Forest_Loop_-_Walking.Deep_Treble_Forest_Loop_-_Walking" 1.0 1.0 0.0 null (`self.As BP Character`))
  (`GameplayStatics.SetBaseSoundMix` "/Game/Music/Mixes/Mute.Mute")
  ;[1 1 1] Create AI Clock
  (bind _returnvalue_6 (`QuartzSubsystem.CreateNewClock` (subsystem `QuartzSubsystem`) "MetronomeAI" (make `QuartzClockSettings` (make `QuartzTimeSignature` 2)) false true))
  (bind _clockhandle_2 (`QuartzClockHandle.SetBeatsPerMinute` :`self` _returnvalue_6 :`BeatsPerMinute` 108.0))
  (set `self.Metronome108` _clockhandle_2)
  ;[1 1 1] Start AI Clock
  (`QuartzClockHandle.StartClock` (`self.Metronome108`))
  (`QuartzClockHandle.SubscribeToQuantizationEvent` (`self.Metronome108`) "Beat" (delegate `Move AI`))
  ;[1 1 1] Create Attack Clock
  (bind _returnvalue_7 (`QuartzSubsystem.CreateNewClock` (subsystem `QuartzSubsystem`) "MetronomeAI" (make `QuartzClockSettings` (make `QuartzTimeSignature` 2)) false true))
  (bind _clockhandle_3 (`QuartzClockHandle.SetBeatsPerMinute` :`self` _returnvalue_7 :`BeatsPerMinute` 108.0))
  (bind _output_get_4 (set `self.MetronomeAI` _clockhandle_3))
  ;[1 1 1] Start Attack Clock
  (`QuartzClockHandle.StartClock` _output_get_4)
  (`QuartzClockHandle.SubscribeToQuantizationEvent` (`self.MetronomeAI`) "Beat" (delegate `Crtical Hit`)))

(event `Beats`
  (params (ClockName :type Name) (QuantizationType :type "EQuartzCommandQuantization Enum" :default "Bar") (NumBars :type Integer) (Beat :type Integer) (BeatFraction :type "Float (single-precision)"))
  ;[1 1 1] Show Beat number
  ;[1 1 1] Allow Dash at Beat 1
  (bind _asbp_character (cast `/Game/Blueprints/BP_Character` (`GameplayStatics.GetPlayerPawn` 0)))
  ;[1 1 1] AI Attack at Beat 1
  (set `/Game/Blueprints/BP_Character.Allow Golem Attack` (== Beat 1) _asbp_character)
  (`KismetSystemLibrary.Delay` (`KismetMathLibrary.Conv_BoolToDouble` (== Beat 2)))
  (set `/Game/Blueprints/BP_Character.Allow Golem Attack` false _asbp_character))

(event `Move AI`
  (params (ClockName :type Name) (QuantizationType :type "EQuartzCommandQuantization Enum" :default "Bar") (NumBars :type Integer) (Beat :type Integer) (BeatFraction :type "Float (single-precision)"))
  (bind _returnvalue (== Beat 1))
  ;[1 1 1] Move AI To Beat 1 (and 3)
  (bind _asbp_character (cast `/Game/Blueprints/BP_Character` (`GameplayStatics.GetPlayerCharacter` 0)))
  (set `/Game/Blueprints/BP_Character.TellAIToMove` _returnvalue _asbp_character)
  ;[1 1 1] Allow Slime AI To Attack On 1 & 3
  (set `/Game/Blueprints/BP_Character.Allow Slime Attack` _returnvalue _asbp_character)
  (set `/Game/Blueprints/BP_Character.Allow Slime Attack` false _asbp_character)
  (set `/Game/Blueprints/BP_Character.Allow Dash` _returnvalue _asbp_character))

(event `Crtical Hit`
  (params (ClockName :type Name) (QuantizationType :type "EQuartzCommandQuantization Enum" :default "Bar") (NumBars :type Integer) (Beat :type Integer) (BeatFraction :type "Float (single-precision)"))
  (bind _returnvalue (== Beat 1))
  (bind _returnvalue_2 (== Beat 2))
  ;[1 1 1] Critical Hit
  (bind _asbp_character (cast `/Game/Blueprints/BP_Character` (`GameplayStatics.GetPlayerCharacter` 0)))
  (set `/Game/Blueprints/BP_Character.Launch` _returnvalue _asbp_character)
  (`KismetSystemLibrary.Delay` (`KismetMathLibrary.Conv_BoolToDouble` _returnvalue_2))
  (set `/Game/Blueprints/BP_Character.Launch` false _asbp_character)
  (`/Engine/EditorBlueprintResources/StandardMacros.DoOnce` false :!label _label
    (:`Completed`
      (set `/Game/Blueprints/BP_Character.Shoot` _returnvalue _asbp_character)
      (`KismetSystemLibrary.Delay` (`KismetMathLibrary.Conv_BoolToDouble` _returnvalue_2))
      (set `/Game/Blueprints/BP_Character.Shoot` false _asbp_character)
      (goto _label :!via `Reset`))))

(fn `UserConstructionScript`)