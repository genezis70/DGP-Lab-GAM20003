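; BP_Slime is a 2D ground enemy that patrols and turns at walls and ledges via overlap triggers.
; TellAIToMove and Attack read flags on BP_Character to gate forward movement and knockback.
; A front trigger toggles AttackPlayer, while the back trigger adds movement along the player's forward vector and sets a fixed yaw.
; Dash speed and flipbook-state functions using player animations are defined but not called here.
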(event `StopAI`
  ;[1 1 1] Stop AI From Moving
  (`self.AddMovementInput` (`self.GetActorForwardVector`) 0.0 true))

(event `MoveForward`
  ;[1 1 1] Make AI Move
  (`self.AddMovementInput` (`self.GetActorForwardVector`)))

(event `self.Walldetector.OnComponentBeginOverlap`
  (params (OverlappedComponent :type "PrimitiveComponent Object Reference") (OtherActor :type "Actor Object Reference") (OtherComp :type "PrimitiveComponent Object Reference") (OtherBodyIndex :type Integer) (bFromSweep :type Boolean) (SweepResult :type "HitResult Structure (by ref)"))
  ;[1 1 1] Detects Walls and Turns AI
  (`self.TurnChar`))

(event `Tell AI To Move`
  ;[1 1 1] Move At Beat 1
  (bind _asbp_character (cast `/Game/Blueprints/BP_Character` (`GameplayStatics.GetPlayerCharacter` 0)))
  (if (`/Game/Blueprints/BP_Character.TellAIToMove` _asbp_character)
    (`self.MoveForward`)
    (else
      (`self.StopAI`))))

(event `Attack`
  (`self.StopAI`)
  (bind _asbp_character (cast `/Game/Blueprints/BP_Character` (`GameplayStatics.GetPlayerCharacter` 0)))
  (if (`/Game/Blueprints/BP_Character.Allow AI Attack` _asbp_character)
    (set `self.Knockback` true)))

(event `self.LedgeDetector.OnComponentEndOverlap`
  (params (OverlappedComponent :type "PrimitiveComponent Object Reference") (OtherActor :type "Actor Object Reference") (OtherComp :type "PrimitiveComponent Object Reference") (OtherBodyIndex :type Integer))
  ;[1 1 1] Detects Ledges and Turns AI
  (`self.TurnChar`))

(event `self.Back.OnComponentBeginOverlap`
  (params (OverlappedComponent :type "PrimitiveComponent Object Reference") (OtherActor :type "Actor Object Reference") (OtherComp :type "PrimitiveComponent Object Reference") (OtherBodyIndex :type Integer) (bFromSweep :type Boolean) (SweepResult :type "HitResult Structure (by ref)"))
  ;[1 1 1] Back
  (bind _asbp_character (cast `/Game/Blueprints/BP_Character` OtherActor))
  (`self.AddMovementInput` (`self.GetActorForwardVector` _asbp_character))
  (`self.K2_SetActorRotation` (struct :`Yaw` 180.0)))

(event `self.Front.OnComponentBeginOverlap`
  (params (OverlappedComponent :type "PrimitiveComponent Object Reference") (OtherActor :type "Actor Object Reference") (OtherComp :type "PrimitiveComponent Object Reference") (OtherBodyIndex :type Integer) (bFromSweep :type Boolean) (SweepResult :type "HitResult Structure (by ref)"))
  (set `self.AttackPlayer` true))

(event `self.Front.OnComponentEndOverlap`
  (params (OverlappedComponent :type "PrimitiveComponent Object Reference") (OtherActor :type "Actor Object Reference") (OtherComp :type "PrimitiveComponent Object Reference") (OtherBodyIndex :type Integer))
  (set `self.AttackPlayer` false))

(fn `F Set Movement States`
  (params (MovementStates :type "/Game/Blueprints/Enums/E_MovementStates Enum" :default "NewEnumerator0"))
  (bind _sprite (`self.Sprite`))
  (bind _sprite_2 (`self.Sprite`))
  (`PaperFlipbookComponent.SetLooping` (`self.Sprite`) (select `/Game/Blueprints/Enums/E_MovementStates` MovementStates :`NewEnumerator0` true :`NewEnumerator1` true :`NewEnumerator2` true :`NewEnumerator5` true :`NewEnumerator6` true))
  (`PaperFlipbookComponent.Play` (`self.Sprite`))
  (switch `/Game/Blueprints/Enums/E_MovementStates` MovementStates
    (:`NewEnumerator0`
      (`PaperFlipbookComponent.SetFlipbook` _sprite "/Game/SunnyLandAssets/sprites/player/idle/FB_player_idle.FB_player_idle"))
    (:`NewEnumerator1`
      (`PaperFlipbookComponent.SetFlipbook` _sprite "/Game/SunnyLandAssets/sprites/player/run/FB_player_run.FB_player_run")
      (`SceneComponent.K2_SetRelativeRotation` _sprite_2 (struct :`Yaw` -180.0) false false))
    (:`NewEnumerator2`
      (`PaperFlipbookComponent.SetFlipbook` _sprite "/Game/SunnyLandAssets/sprites/player/run/FB_player_run.FB_player_run")
      (`SceneComponent.K2_SetRelativeRotation` :`self` _sprite_2))
    (:`NewEnumerator5`
      (`PaperFlipbookComponent.SetFlipbook` _sprite "/Game/SunnyLandAssets/sprites/player/run/FB_player_dash.FB_player_dash")
      (`SceneComponent.K2_SetRelativeRotation` _sprite_2 (struct :`Yaw` -180.0) false false))
    (:`NewEnumerator6`
      (`PaperFlipbookComponent.SetFlipbook` _sprite "/Game/SunnyLandAssets/sprites/player/run/FB_player_dash.FB_player_dash")
      (`SceneComponent.K2_SetRelativeRotation` :`self` _sprite_2))
    (:`NewEnumerator3`
      (`PaperFlipbookComponent.SetFlipbook` _sprite "/Game/SunnyLandAssets/sprites/player/jump/FB_player_fall.FB_player_fall"))))

(fn `StartDash`
  (set `CharacterMovementComponent.MaxWalkSpeed` (`self.DashSpeed`) (`self.CharacterMovement`))
  (set `self.Dash` true))

(fn `StopDash`
  (set `CharacterMovementComponent.MaxWalkSpeed` (`self.WalkSpeed`) (`self.CharacterMovement`))
  (set `self.Dash` false))

(fn `TurnChar`
  (`self.K2_SetActorRotation` (`KismetMathLibrary.ComposeRotators` (`self.K2_GetActorRotation`) (struct :`Yaw` 180.0))))

(fn `UserConstructionScript`)