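; BP_Block_Deactivated is a sprite block that toggles between on and off when hit by a violin note.
; Each BP_Violin_Note2 overlapping BlockCol is destroyed, and a FlipFlop swaps the Block sprite between blue note on and off.
; After a short delay, a second FlipFlop prints the state and moves the actor along Y, keeping X and Z, to shift it between two depths.
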(event `self.BlockCol.OnComponentBeginOverlap`
  (params (OverlappedComponent :type "PrimitiveComponent Object Reference") (OtherActor :type "Actor Object Reference") (OtherComp :type "PrimitiveComponent Object Reference") (OtherBodyIndex :type Integer) (bFromSweep :type Boolean) (SweepResult :type "HitResult Structure (by ref)"))
  (bind (_returnvalue_x _returnvalue_y _returnvalue_z) (`KismetMathLibrary.BreakVector` (`self.K2_GetActorLocation`)))
  (bind _asbp_violin_note_2 (cast `/Game/Blueprints/BP_Violin_Note2` OtherActor))
  (`self.K2_DestroyActor` _asbp_violin_note_2)
  (`/Engine/EditorBlueprintResources/StandardMacros.FlipFlop`
    (:`A`
      (`PaperSpriteComponent.SetSprite` (`self.Block`) "/Game/sarah_assets/music_sprites/S_blue_note_on.S_blue_note_on"))
    (:`B`
      (`PaperSpriteComponent.SetSprite` (`self.Block`) "/Game/sarah_assets/music_sprites/T_blue_note_off_Sprite.T_blue_note_off_Sprite")))
  (`KismetSystemLibrary.Delay` 0.2)
  (`/Engine/EditorBlueprintResources/StandardMacros.FlipFlop`
    (:`A`
      (`KismetSystemLibrary.PrintString` "on")
      (`self.K2_SetActorLocation` (`KismetMathLibrary.MakeVector` _returnvalue_x 0.0 _returnvalue_z)))
    (:`B`
      (`KismetSystemLibrary.PrintString` "off")
      (`self.K2_SetActorLocation` (`KismetMathLibrary.MakeVector` _returnvalue_x -25.0 _returnvalue_z)))))

(fn `UserConstructionScript`)