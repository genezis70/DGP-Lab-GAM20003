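; SheetMusic is a pickup actor that floats vertically and disappears when a BP_Character overlaps it.
; On BeginPlay a timeline starts at a play rate of one over FloatCycleLength, lerping the actor's Z between TopPoint and BottomPoint while keeping X and Y.
; The overlap handler only destroys the actor and passes nothing to the character.
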(event `self.ReceiveActorBeginOverlap`
  (params (OtherActor :type "Actor Object Reference"))
  (cast `/Game/Blueprints/BP_Character` OtherActor)
  (`self.K2_DestroyActor`))

(event `self.ReceiveBeginPlay`
  (bind _returnvalue (`ActorComponent.GetOwner` (`self.SheetMusic`)))
  (bind (_returnvalue_x _returnvalue_y) (`KismetMathLibrary.BreakVector` (`self.K2_GetActorLocation` _returnvalue)))
  (`TimelineComponent.SetPlayRate` (`self.Timeline`) (/ 1.0 (`self.Float Cycle Length`)))
  (bind (_direction _float_timing_checkpoint) (`Timeline|Timeline`)
    (:`Update`
      (`self.K2_SetActorLocation` _returnvalue (`KismetMathLibrary.MakeVector` _returnvalue_x _returnvalue_y (`KismetMathLibrary.Lerp` (`self.Top Point`) (`self.Bottom Point`) _float_timing_checkpoint)) false false))))

(fn `UserConstructionScript`)