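; BP_ViolinNote is a note actor that toggles block collision on overlap and destroys itself when it touches a Paper2D tile map.
; Its Collision overlap event casts the other actor to BP_Block and uses a FlipFlop to alternate that block's Box between query-only and query-and-physics collision, printing debug text.
; The FlipFlop state lives on the note rather than the block, and unconnected SetActorLocation nodes remain unused.
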(event `self.collision.OnComponentBeginOverlap`
  (params (OverlappedComponent :type "PrimitiveComponent Object Reference") (OtherActor :type "Actor Object Reference") (OtherComp :type "PrimitiveComponent Object Reference") (OtherBodyIndex :type Integer) (bFromSweep :type Boolean) (SweepResult :type "HitResult Structure (by ref)"))
  (cast `PaperTileMapActor` OtherActor
    (:`then`
      (`self.K2_DestroyActor`))
    (:`CastFailed`
      (bind _asbp_block (cast `/Game/Blueprints/BP_Block` OtherActor))
      (`/Engine/EditorBlueprintResources/StandardMacros.FlipFlop`
        (:`A`
          (`PrimitiveComponent.SetCollisionEnabled` (`/Game/Blueprints/BP_Block.Box` _asbp_block) "QueryOnly")
          (`KismetSystemLibrary.PrintString` "off"))
        (:`B`
          (`PrimitiveComponent.SetCollisionEnabled` (`/Game/Blueprints/BP_Block.Box` _asbp_block) "QueryAndPhysics")
          (`KismetSystemLibrary.PrintString` "on"))))))

(fn `UserConstructionScript`)