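; BP_trampoline is a 2D sprite trampoline that launches the player character upward on contact.
; A box overlap matching the player reference fires a DoOnce-gated launch that overrides vertical velocity, plays a bounce sound and shows the pressed sprite.
; After a delay, it restores the reset sprite and reopens the gate for the next bounce.
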(event `self.Box.OnComponentBeginOverlap`
  (params (OverlappedComponent :type "PrimitiveComponent Object Reference") (OtherActor :type "Actor Object Reference") (OtherComp :type "PrimitiveComponent Object Reference") (OtherBodyIndex :type Integer) (bFromSweep :type Boolean) (SweepResult :type "HitResult Structure (by ref)"))
  (if (== OtherActor (`self.PlayerCharacterRef`))
    (`/Engine/EditorBlueprintResources/StandardMacros.DoOnce` false :!label _label
      (:`Completed`
        (`Character.LaunchCharacter` (`self.PlayerCharacterRef`) (`KismetMathLibrary.MakeVector` 0.0 0.0 (`self.Launch Velocity Z`)) false true)
        (`GameplayStatics.PlaySound2D` "/Game/Sounds/accent_bounce.accent_bounce" 1.0 1.0 0.0 null null)
        (`PaperSpriteComponent.SetSprite` (`self.PaperSprite`) "/Game/sarah_assets/music_sprites/accent_pressed_Sprite.accent_pressed_Sprite")
        (`KismetSystemLibrary.Delay` (`self.Duration`))
        (`PaperSpriteComponent.SetSprite` (`self.PaperSprite`) "/Game/sarah_assets/music_sprites/trampoline_reset.trampoline_reset")
        (`self.resetTrampoline`)))))

(event `resetTrampoline`
  (goto _label :!via `Reset`))

(fn `UserConstructionScript`
  (`parent.UserConstructionScript`))