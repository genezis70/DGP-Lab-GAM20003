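; BP_SheetMusic is a collectible sheet music pickup that floats vertically and counts toward clearing the level.
; On overlap with BP_Character it increments and prints the character's collected count.
; At exactly three it sets and prints Levelclear without destroying itself; otherwise it destroys itself.
; From BeginPlay, a Timeline scaled by FloatCycleLength lerps its Z between TopPoint and BottomPoint.
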(event `self.SheetMusic.OnComponentBeginOverlap`
  (params (OverlappedComponent :type "PrimitiveComponent Object Reference") (OtherActor :type "Actor Object Reference") (OtherComp :type "PrimitiveComponent Object Reference") (OtherBodyIndex :type Integer) (bFromSweep :type Boolean) (SweepResult :type "HitResult Structure (by ref)"))
  (bind _asbp_character (cast `/Game/Blueprints/BP_Character` OtherActor))
  (bind _output_get (set `/Game/Blueprints/BP_Character.SheetmusicCollected` (+ (`/Game/Blueprints/BP_Character.SheetmusicCollected` _asbp_character) 1.0) _asbp_character))
  (`KismetSystemLibrary.PrintString` (`KismetStringLibrary.Conv_DoubleToString` _output_get))
  (if (== _output_get 3.0)
    (bind _output_get_2 (set `/Game/Blueprints/BP_Character.Levelclear` true _asbp_character))
    (`KismetSystemLibrary.PrintString` (`KismetStringLibrary.Conv_BoolToString` _output_get_2))
    (else
      (`self.K2_DestroyActor`))))

(event `self.ReceiveBeginPlay`
  (bind _returnvalue (`ActorComponent.GetOwner` (`self.SheetMusic`)))
  (bind (_returnvalue_x _returnvalue_y) (`KismetMathLibrary.BreakVector` (`self.K2_GetActorLocation` _returnvalue)))
  (`TimelineComponent.SetPlayRate` (`self.Timeline`) (/ 1.0 (`self.Float Cycle Length`)))
  (bind (_direction _float_timing_checkpoint) (`Timeline|Timeline`)
    (:`Update`
      (`self.K2_SetActorLocation` _returnvalue (`KismetMathLibrary.MakeVector` _returnvalue_x _returnvalue_y (`KismetMathLibrary.Lerp` (`self.Top Point`) (`self.Bottom Point`) _float_timing_checkpoint)) false false))))

(fn `UserConstructionScript`)