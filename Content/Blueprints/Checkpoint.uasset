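; Checkpoint actor that sets a character's respawn location when a BP_Character overlaps its box.
; It starts with one sprite and switches to another on overlap, storing its current position as the respawn point.
; A timeline started at BeginPlay, rate-scaled by a cycle length, moves the whole actor vertically by lerping its world Z between top and bottom points.
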(event `self.Box.OnComponentBeginOverlap`
  (params (OverlappedComponent :type "PrimitiveComponent Object Reference") (OtherActor :type "Actor Object Reference") (OtherComp :type "PrimitiveComponent Object Reference") (OtherBodyIndex :type Integer) (bFromSweep :type Boolean) (SweepResult :type "HitResult Structure (by ref)"))
  (bind _asbp_character (cast `/Game/Blueprints/BP_Character` OtherActor))
  (set `/Game/Blueprints/BP_Character.Respawn Location` (`self.K2_GetActorLocation`) _asbp_character)
  (`PaperSpriteComponent.SetSprite` (`self.Checkpoint`) "/Game/sarah_assets/checkpoint_asset/T_crochet_Sprite.T_crochet_Sprite"))

(event `self.ReceiveBeginPlay`
  (bind _returnvalue (`ActorComponent.GetOwner` (`self.Checkpoint`)))
  (bind (_returnvalue_x _returnvalue_y) (`KismetMathLibrary.BreakVector` (`self.K2_GetActorLocation` _returnvalue)))
  (`PaperSpriteComponent.SetSprite` (`self.Checkpoint`) "/Game/sarah_assets/checkpoint_asset/T_crochet1_Sprite.T_crochet1_Sprite")
  (`TimelineComponent.SetPlayRate` (`self.Timeline`) (/ 1.0 (`self.Float Cycle Length`)))
  (bind (_direction _float_timing_checkpoint) (`Timeline|Timeline`)
    (:`Update`
      (`self.K2_SetActorLocation` _returnvalue (`KismetMathLibrary.MakeVector` _returnvalue_x _returnvalue_y (`KismetMathLibrary.Lerp` (`self.Top Point`) (`self.Bottom Point`) _float_timing_checkpoint)) false false))))

(fn `UserConstructionScript`)