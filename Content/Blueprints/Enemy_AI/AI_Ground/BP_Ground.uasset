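; BP_Ground is a 2D ground enemy with snake sprites that moves forward or stops according to the player character's TellAIToMove beat flag.
; Wall and ledge overlaps, plus hits against slimes or golems, flip it around; damage drains GroundLives until it is destroyed.
; Attack, gated by the player's AllowGolemAttack, applies damage and uses a sphere trace to launch the player away.
; Dash and movement-state functions using player flipbooks are never called here.
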(event `StopAI`
  ;[1 1 1] Stop AI From Moving
  (`self.AddMovementInput` (`self.GetActorForwardVector`) 0.0 true)
  (`PaperFlipbookComponent.SetFlipbook` (`self.Sprite`) "/Game/KaI_Assets/snake/snake_IDLE.snake_IDLE"))

(event `MoveForward`
  ;[1 1 1] Make AI Move
  (`self.AddMovementInput` (`self.GetActorForwardVector`))
  (`PaperFlipbookComponent.SetFlipbook` (`self.Sprite`) "/Game/KaI_Assets/snake/snake_IDLE.snake_IDLE"))

(event `self.Walldetector.OnComponentBeginOverlap`
  (params (OverlappedComponent :type "PrimitiveComponent Object Reference") (OtherActor :type "Actor Object Reference") (OtherComp :type "PrimitiveComponent Object Reference") (OtherBodyIndex :type Integer) (bFromSweep :type Boolean) (SweepResult :type "HitResult Structure (by ref)"))
  ;[1 1 1] Detects Walls and Turns AI
  (`self.TurnChar`))

(event `Tell AI To Move`
  ;[1 1 1] Move At Beat 1
  (bind _asbp_character (cast `/Game/Blueprints/BP_Character` (`GameplayStatics.GetPlayerCharacter` 0)))
  (if (`/Game/Blueprints/BP_Character.TellAIToMove` _asbp_character)
    (`self.MoveForward`)
    (else
      (`self.StopAI`))))

(event `self.ReceiveAnyDamage`
  (params (Damage :type "Float (single-precision)") (DamageType :type "DamageType Object Reference") (InstigatedBy :type "Controller Object Reference") (DamageCauser :type "Actor Object Reference"))
  (bind _output_get (set `self.Ground Lives` (`KismetMathLibrary.FClamp` (- (`self.Ground Lives`) Damage) 0.0 (`self.Ground Lives Max`))))
  (if (== _output_get 0.0)
    (`self.K2_DestroyActor`)))

(event `self.LedgeDetector.OnComponentEndOverlap`
  (params (OverlappedComponent :type "PrimitiveComponent Object Reference") (OtherActor :type "Actor Object Reference") (OtherComp :type "PrimitiveComponent Object Reference") (OtherBodyIndex :type Integer))
  ;[1 1 1] Detects Ledges and Turns AI
  (`self.TurnChar`))

(event `self.Back.OnComponentBeginOverlap`
  (params (OverlappedComponent :type "PrimitiveComponent Object Reference") (OtherActor :type "Actor Object Reference") (OtherComp :type "PrimitiveComponent Object Reference") (OtherBodyIndex :type Integer) (bFromSweep :type Boolean) (SweepResult :type "HitResult Structure (by ref)"))
  ;[1 1 1] Back
  (bind _asbp_character (cast `/Game/Blueprints/BP_Character` OtherActor))
  (`self.AddMovementInput` (`self.GetActorForwardVector` _asbp_character))
  (`self.K2_SetActorRotation` (struct :`Yaw` 180.0)))

(event `Attack`
  (bind _returnvalue_x (`KismetMathLibrary.BreakVector` (`self.K2_GetActorLocation`)))
  (bind _returnvalue (`self.K2_GetActorLocation` self))
  (bind _asbp_character (cast `/Game/Blueprints/BP_Character` (`GameplayStatics.GetPlayerCharacter` 0)))
  (if (`/Game/Blueprints/BP_Character.Allow Golem Attack` _asbp_character)
    (bind _returnvalue_2 (`GameplayStatics.ApplyDamage` _asbp_character (`self.Base Damage`) null self))
    (`KismetSystemLibrary.PrintString` (`KismetStringLibrary.Conv_DoubleToString` _returnvalue_2))
    (bind (_outhit _returnvalue_3) (`KismetSystemLibrary.SphereTraceSingleForObjects` :`Start` _returnvalue :`End` (+ _returnvalue (* (`self.GetActorForwardVector` self) 1.0)) :`Radius` 15.0 :`ObjectTypes` (`|MakeArray` "ObjectTypeQuery3" :!type "EObjectTypeQuery Enum") :`DrawDebugType` "ForDuration"))
    (if _returnvalue_3
      (bind _asbp_character_2 (cast `/Game/Blueprints/BP_Character` (`.HitActor` (`GameplayStatics.BreakHitResult` _outhit))))
      (bind _returnvalue_x_2 (`KismetMathLibrary.BreakVector` (`self.K2_GetActorLocation` _asbp_character_2)))
      (if (> _returnvalue_x _returnvalue_x_2)
        (`self.LaunchCharacter` _asbp_character_2 (-100.0 0.0 100.0) false false)
        (else
          (`self.LaunchCharacter` _asbp_character_2 (100.0 0.0 100.0) false false))))))

(event `self.Front.OnComponentBeginOverlap`
  (params (OverlappedComponent :type "PrimitiveComponent Object Reference") (OtherActor :type "Actor Object Reference") (OtherComp :type "PrimitiveComponent Object Reference") (OtherBodyIndex :type Integer) (bFromSweep :type Boolean) (SweepResult :type "HitResult Structure (by ref)"))
  (cast `/Game/Blueprints/BP_Character` OtherActor)
  (set `self.Knockback` true))

(event `self.Front.OnComponentEndOverlap`
  (params (OverlappedComponent :type "PrimitiveComponent Object Reference") (OtherActor :type "Actor Object Reference") (OtherComp :type "PrimitiveComponent Object Reference") (OtherBodyIndex :type Integer))
  (cast `/Game/Blueprints/BP_Character` OtherActor)
  (set `self.Knockback` false))

(event `self.CapsuleComponent.OnComponentHit`
  (params (HitComponent :type "PrimitiveComponent Object Reference") (OtherActor :type "Actor Object Reference") (OtherComp :type "PrimitiveComponent Object Reference") (NormalImpulse :type "Vector Structure") (Hit :type "HitResult Structure (by ref)"))
  (cast `/Game/Blueprints/Enemy_AI/AI_Ground/Slime/BP_Slime` OtherActor
    (:`then`
      (`self.TurnChar`))
    (:`CastFailed`
      (cast `/Game/Blueprints/Enemy_AI/AI_Ground/BP_Golem` OtherActor)
      (`self.TurnChar`))))

(fn `F Set Movement States`
  (params (MovementStates :type "/Game/Blueprints/Enums/E_MovementStates Enum" :default "NewEnumerator0"))
  (bind _sprite (`self.Sprite`))
  (bind _sprite_2 (`self.Sprite`))
  (`PaperFlipbookComponent.SetLooping` (`self.Sprite`) (select `/Game/Blueprints/Enums/E_MovementStates` MovementStates :`NewEnumerator0` true :`NewEnumerator1` true :`NewEnumerator2` true :`NewEnumerator5` true :`NewEnumerator6` true))
  (`PaperFlipbookComponent.Play` (`self.Sprite`))
  (switch `/Game/Blueprints/Enums/E_MovementStates` MovementStates
    (:`NewEnumerator0`
      (`PaperFlipbookComponent.SetFlipbook` _sprite "/Game/SunnyLandAssets/sprites/player/idle/FB_player_idle.FB_player_idle"))
    (:`NewEnumerator1`
      (`PaperFlipbookComponent.SetFlipbook` _sprite "/Game/SunnyLandAssets/sprites/player/run/FB_player_run.FB_player_run")
      (`SceneComponent.K2_SetRelativeRotation` _sprite_2 (struct :`Yaw` -180.0) false false))
    (:`NewEnumerator2`
      (`PaperFlipbookComponent.SetFlipbook` _sprite "/Game/SunnyLandAssets/sprites/player/run/FB_player_run.FB_player_run")
      (`SceneComponent.K2_SetRelativeRotation` :`self` _sprite_2))
    (:`NewEnumerator5`
      (`PaperFlipbookComponent.SetFlipbook` _sprite "/Game/SunnyLandAssets/sprites/player/run/FB_player_dash.FB_player_dash")
      (`SceneComponent.K2_SetRelativeRotation` _sprite_2 (struct :`Yaw` -180.0) false false))
    (:`NewEnumerator6`
      (`PaperFlipbookComponent.SetFlipbook` _sprite "/Game/SunnyLandAssets/sprites/player/run/FB_player_dash.FB_player_dash")
      (`SceneComponent.K2_SetRelativeRotation` :`self` _sprite_2))
    (:`NewEnumerator3`
      (`PaperFlipbookComponent.SetFlipbook` _sprite "/Game/SunnyLandAssets/sprites/player/jump/FB_player_fall.FB_player_fall"))))

(fn `StartDash`
  (set `CharacterMovementComponent.MaxWalkSpeed` (`self.DashSpeed`) (`self.CharacterMovement`))
  (set `self.Dash` true))

(fn `StopDash`
  (set `CharacterMovementComponent.MaxWalkSpeed` (`self.WalkSpeed`) (`self.CharacterMovement`))
  (set `self.Dash` false))

(fn `TurnChar`
  (`self.K2_SetActorRotation` (`KismetMathLibrary.ComposeRotators` (`self.K2_GetActorRotation`) (struct :`Yaw` 180.0))))

(fn `UserConstructionScript`)